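; Test actor Blueprint that drives a fluid-style LBM (likely Lattice Boltzmann) simulation for debugging.
; BeginPlay updates resources, sets the initial LBM state and fetches a debug value from the output texture.
; While simulating, each Tick runs streaming, then collision, then the debug texture readback.
; Debug keys start, pause or single-step the simulation; an EndRenderdoc call is left unconnected.
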(event EventBeginPlay
  (Development|PrintText "Test BP")
  (Class|SimulationLibrary|UpdateResource)
  (Class|SimulationLibrary|LBMInitialState)
  (Class|SimulationLibrary|GetDebugTextureValue (Variables|Default|GetOutTexture)))

(event Collision|EventActorBeginOverlap
  (params (OtherActor :type Actor%20Object%20Reference)))

(event EventTick
  (params (DeltaSeconds :type Float%20%28single-precision%29))
  (if (Variables|Default|GetSimulating)
    (Development|PrintString "Step")
    (Class|SimulationLibrary|LBMStreaming)
    (Class|SimulationLibrary|LBMCollision)
    (Class|SimulationLibrary|GetDebugTextureValue (Variables|Default|GetOutTexture))))

(event Input|KeyboardEvents|DebugKey1
  (params (Key :type Key%20Structure :default "None") (ActionValue :type Input%20Action%20Value%20Structure))
  (:Pressed
    (Development|PrintString "Start Sim")
    (Variables|Default|SetSimulating true)))

(event Input|KeyboardEvents|DebugKey2
  (params (Key :type Key%20Structure :default "None") (ActionValue :type Input%20Action%20Value%20Structure))
  (:Pressed
    (Development|PrintString "Pause Sim")
    (Variables|Default|SetSimulating false)))

(event Input|KeyboardEvents|DebugKey3
  (params (Key :type Key%20Structure :default "None") (ActionValue :type Input%20Action%20Value%20Structure))
  (:Pressed
    (Development|PrintString "Step")
    (Class|SimulationLibrary|LBMStreaming)
    (Class|SimulationLibrary|LBMCollision)
    (Class|SimulationLibrary|GetDebugTextureValue (Variables|Default|GetOutTexture))))

(fn ConstructionScript)