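; Demo pipeline actor that controls a volumetric Niagara effect, keeping it idle until a debug key starts it.
; The construction script moves the Niagara component to the Origin world position with no rotation and unit scale, and passes Origin into the system as a parameter.
; BeginPlay zeroes the particle spawn rate, and pressing DebugKey8 raises it to a high fixed value, with no logic to switch it back off.
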(event EventBeginPlay
  (Niagara|SetNiagaraVariable(Float) (Variables|Default|GetVolumetricNiagaraSystem_Final) "Particle Spawn Rate" (Math|Float|MakeLiteralFloat 0.0)))

(event Collision|EventActorBeginOverlap
  (params (OtherActor :type Actor%20Object%20Reference)))

(event EventTick
  (params (DeltaSeconds :type Float%20%28single-precision%29)))

(event Input|KeyboardEvents|DebugKey8
  (params (Key :type Key%20Structure :default "None") (ActionValue :type Input%20Action%20Value%20Structure))
  (:Pressed
    (Niagara|SetNiagaraVariable(Float) (Variables|Default|GetVolumetricNiagaraSystem_Final) "Particle Spawn Rate" (Math|Float|MakeLiteralFloat 1.2e+04))))

(fn ConstructionScript
  (bind _origin (Variables|Default|GetOrigin))
  (Transformation|SetWorldTransform (Variables|Default|GetVolumetricNiagaraSystem_Final) (Math|Transform|MakeTransform _origin) false false)
  (Class|NiagaraComponent|SetNiagaraVariableVec3 (Variables|Default|GetVolumetricNiagaraSystem_Final) "Origin" _origin))