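; Demo pipeline actor that feeds a simulation's 3D texture and world bounds to a Niagara vector field component.
; The construction script passes the SimBoundWorld min and max to the system as BoundMinWorld and BoundMaxWorld.
; It also sends SimTex3D, though that texture variable name is set to None.
; The component's world transform is reset to identity, independent of the actor's placement.
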(fn `UserConstructionScript`
  (bind _n_vectorfield (`self.N_VectorField`))
  (bind (_min _max) (break `Box` (`self.SimBoundWorld`)))
  (`NiagaraComponent.SetVariableVec3` _n_vectorfield "BoundMinWorld" _min)
  (`NiagaraComponent.SetVariableVec3` _n_vectorfield "BoundMaxWorld" _max)
  (`NiagaraComponent.SetVariableTexture` (`self.N_VectorField`) "None" (`self.SimTex3D`))
  (`SceneComponent.K2_SetWorldTransform` (`self.N_VectorField`) (`KismetMathLibrary.MakeTransform` (0.0 0.0 0.0)) false false))