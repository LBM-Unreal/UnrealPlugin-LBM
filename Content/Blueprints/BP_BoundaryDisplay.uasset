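; Editor-time display of a simulation volume's six outer boundary faces, colored by boundary condition: no-slip, inflow, outflow or free-slip.
; The construction script loops over Boundaries, and SetOuterBoundary assigns the matching material to the BoundaryDisplay child mesh at that index, so child order matters.
; The same loop body also fits six thin, scaled meshes onto the faces of the SimBoundWorld box.
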(fn `SetOuterBoundary`
  (params (FaceIndex :type Integer) (BoundaryType :type Integer))
  (bind _asstatic_mesh_component (cast `StaticMeshComponent` (`SceneComponent.GetChildComponent` (`self.BoundaryDisplay`) FaceIndex)))
  (switch `int` BoundaryType
    (:`1`
      (`PrimitiveComponent.SetMaterial` _asstatic_mesh_component 0 "/Game/Visualization/MI_NoSlip.MI_NoSlip"))
    (:`2`
      (`PrimitiveComponent.SetMaterial` _asstatic_mesh_component 0 "/Game/Visualization/MI_Inflow.MI_Inflow"))
    (:`3`
      (`PrimitiveComponent.SetMaterial` _asstatic_mesh_component 0 "/Game/Visualization/MI_Outflow.MI_Outflow"))
    (:`4`
      (`PrimitiveComponent.SetMaterial` _asstatic_mesh_component 0 "/Game/Visualization/MI_FreeSlip.MI_FreeSlip"))))

(fn `UserConstructionScript`
  (bind _simboundworld (`self.SimBoundWorld`))
  (bind (_min _max) (break `Box` _simboundworld))
  (bind _x (.x (/ (`KismetMathLibrary.GetBoxSize` _simboundworld) (100.0 100.0 100.0))))
  (bind _y (.y (/ (`KismetMathLibrary.GetBoxSize` _simboundworld) (100.0 100.0 100.0))))
  (bind _z (.z (/ (`KismetMathLibrary.GetBoxSize` _simboundworld) (100.0 100.0 100.0))))
  (bind _x_2 (.x (* (+ _max _min) (0.5 0.5 0.5))))
  (bind _y_2 (.y (* (+ _max _min) (0.5 0.5 0.5))))
  (bind _z_2 (.z (* (+ _max _min) (0.5 0.5 0.5))))
  (for (_array_element _array_index) (`self.Boundaries`)
    (`self.SetOuterBoundary` _array_index _array_element)
    ; Initialize Boundary visualize planes
    (`SceneComponent.K2_SetWorldTransform` (`self.B_Top`) (`KismetMathLibrary.MakeTransform` (`KismetMathLibrary.MakeVector` _x_2 _y_2 (.z _max)) (struct) (`KismetMathLibrary.MakeVector` _x _y 0.01)) false false)
    (`SceneComponent.K2_SetWorldTransform` (`self.B_Bottom`) (`KismetMathLibrary.MakeTransform` (`KismetMathLibrary.MakeVector` _x_2 _y_2 (.z _min)) (struct) (`KismetMathLibrary.MakeVector` _x _y 0.01)) false false)
    (`SceneComponent.K2_SetWorldTransform` (`self.B_Front`) (`KismetMathLibrary.MakeTransform` (`KismetMathLibrary.MakeVector` (.x _max) _y_2 _z_2) (struct) (`KismetMathLibrary.MakeVector` 0.01 _y _z)) false false)
    (`SceneComponent.K2_SetWorldTransform` (`self.B_Back`) (`KismetMathLibrary.MakeTransform` (`KismetMathLibrary.MakeVector` (.x _min) _y_2 _z_2) (struct) (`KismetMathLibrary.MakeVector` 0.01 _y _z)) false false)
    (`SceneComponent.K2_SetWorldTransform` (`self.B_Right`) (`KismetMathLibrary.MakeTransform` (`KismetMathLibrary.MakeVector` _x_2 (.y _max) _z_2) (struct) (`KismetMathLibrary.MakeVector` _x 0.01 _z)) false false)
    (`SceneComponent.K2_SetWorldTransform` (`self.B_Left`) (`KismetMathLibrary.MakeTransform` (`KismetMathLibrary.MakeVector` _x_2 (.y _min) _z_2) (struct) (`KismetMathLibrary.MakeVector` _x 0.01 _z)) false false)))