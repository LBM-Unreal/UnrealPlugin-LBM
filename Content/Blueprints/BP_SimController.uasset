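; Controller Blueprint for a 3D lattice Boltzmann (LBM) fluid simulation, driven by a UI_SimControl widget and debug keys.
; BeginPlay resizes the 3D texture, binds widget inputs for velocity, density, relaxation and display slice, then initializes the simulation.
; Start, pause, step and reset control it; while simulating, each Tick runs one streaming-collision step and refreshes the debug slice texture.
; A mesh voxelization call is present but never runs.
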(event Custom|OnValueChanged_Event
  (params (InValue :type Float%20%28single-precision%29))
  ;[0.15 0.15 0.15 0.5] UI Button Events
  (Variables|Default|SetDisplaySlice (Math|Float|Truncate InValue)))

(event Custom|OnClicked_Event
  ;[0.15 0.15 0.15 0.5] UI Button Events
  (Development|PrintString "Start Sim")
  (Variables|Default|SetSimulating true))

(event Custom|EventVeloSPChanged
  (params (InValue :type Float%20%28single-precision%29))
  ;[0.15 0.15 0.15 0.5] UI Button Events
  (Variables|Default|SetInitialVelocity InValue))

(event Custom|EventDensSPChanged
  (params (InValue :type Float%20%28single-precision%29))
  ;[0.15 0.15 0.15 0.5] UI Button Events
  (Variables|Default|SetInitialDensity InValue))

(event Custom|EventRelaxSPChanged
  (params (InValue :type Float%20%28single-precision%29))
  ;[0.15 0.15 0.15 0.5] UI Button Events
  (Variables|Default|SetRelaxationFactor InValue))

(event Custom|OnClicked_Event_0
  ;[0.15 0.15 0.15 0.5] UI Button Events
  (Development|PrintString "Pause Sim")
  (Variables|Default|SetSimulating false))

(event Custom|OnClicked_Event_1
  ;[0.15 0.15 0.15 0.5] UI Button Events
  ;[0.15 0.15 0.15 0.5] Simulation Step
  (Development|PrintString "Step")
  (Class|SimulationLibrary|LBMHOMEStreamingCollision3D (Variables|Default|GetDisplaySlice))
  (Class|SimulationLibrary|GetDebugTextureValue3D (Variables|Default|GetOutDebugTex2D)))

(event Custom|OnClicked_Event_2
  (Class|SimulationLibrary|LBMMRInitialState3D (Variables|Default|GetDisplaySlice))
  ;[0.15 0.15 0.15 0.5] Reset Simulation Data
  (Class|SimulationLibrary|GetDebugTextureValue3D (Variables|Default|GetOutDebugTex2D)))

(event EventBeginPlay
  (if (Utilities|IsValid (Variables|Default|GetOutDebugTex2D))
    (if (Utilities|IsValid (Variables|Default|GetOutTex3D))
      (Development|PrintText "Init Sim Resource")
      (Class|SimulationLibrary|UpdateResource3D (Variables|Default|GetSimDim) (Variables|Default|GetOutTex3D)) ; Resize Sim Resources
      ;[0.15 0.15 0.15 0.5] Add Gameplay UI
      (bind _returnvalue (UserInterface|CreateWidget "/Game/Blueprints/UI_SimControl.UI_SimControl_C"))
      (bind _output_get (Variables|Default|SetUIController _returnvalue))
      (UserInterface|Viewport|AddtoViewport _output_get 0)
      (Variables|Default|SetInitialVelocity (Variables|/Script/UMG.SpinBox|GetValue (Variables|/Game/Blueprints/UI_SimControl.UI_SimControl_C|GetVeloSP (Variables|Default|GetUIController))))
      (Variables|Default|SetInitialDensity (Variables|/Script/UMG.SpinBox|GetValue (Variables|/Game/Blueprints/UI_SimControl.UI_SimControl_C|GetDensSP (Variables|Default|GetUIController))))
      (Variables|Default|SetRelaxationFactor (Variables|/Script/UMG.SpinBox|GetValue (Variables|/Game/Blueprints/UI_SimControl.UI_SimControl_C|GetRelaxationSP (Variables|Default|GetUIController))))
      (Variables|Default|SetDisplaySlice (Math|Float|Truncate (Variables|/Script/UMG.SpinBox|GetValue (Variables|/Game/Blueprints/UI_SimControl.UI_SimControl_C|GetDisplaySliceSP (Variables|Default|GetUIController)))))
      (EventDispatchers|AssignOnValueChanged (Variables|/Game/Blueprints/UI_SimControl.UI_SimControl_C|GetVeloSP (Variables|Default|GetUIController)) (delegate Custom|EventVeloSPChanged))
      (EventDispatchers|AssignOnValueChanged (Variables|/Game/Blueprints/UI_SimControl.UI_SimControl_C|GetDensSP (Variables|Default|GetUIController)) (delegate Custom|EventDensSPChanged))
      (EventDispatchers|AssignOnValueChanged (Variables|/Game/Blueprints/UI_SimControl.UI_SimControl_C|GetRelaxationSP (Variables|Default|GetUIController)) (delegate Custom|EventRelaxSPChanged))
      (EventDispatchers|AssignOnValueChanged (Variables|/Game/Blueprints/UI_SimControl.UI_SimControl_C|GetDisplaySliceSP (Variables|Default|GetUIController)) (delegate Custom|OnValueChanged_Event))
      (EventDispatchers|AssignOnClicked (Variables|/Game/Blueprints/UI_SimControl.UI_SimControl_C|GetStartOptimBtn (Variables|Default|GetUIController)) (delegate Custom|OnClicked_Event))
      (EventDispatchers|AssignOnClicked (Variables|/Game/Blueprints/UI_SimControl.UI_SimControl_C|GetStopOptimBtn (Variables|Default|GetUIController)) (delegate Custom|OnClicked_Event_0))
      (EventDispatchers|AssignOnClicked (Variables|/Game/Blueprints/UI_SimControl.UI_SimControl_C|GetOptimizeStepBtn (Variables|Default|GetUIController)) (delegate Custom|OnClicked_Event_1))
      (EventDispatchers|AssignOnClicked (Variables|/Game/Blueprints/UI_SimControl.UI_SimControl_C|GetResetBtn (Variables|Default|GetUIController)) (delegate Custom|OnClicked_Event_2))
      (Class|SimulationLibrary|LBMMRInitialState3D (Variables|Default|GetDisplaySlice))
      ;[0.15 0.15 0.15 0.5] Reset Simulation Data
      (Class|SimulationLibrary|GetDebugTextureValue3D (Variables|Default|GetOutDebugTex2D))
      (else
        (Development|PrintString "Error: Tex3D not set")))
    (else
      (Development|PrintString "Error: OutTexture not set"))))

(event Collision|EventActorBeginOverlap
  (params (OtherActor :type Actor%20Object%20Reference)))

(event EventTick
  (params (DeltaSeconds :type Float%20%28single-precision%29))
  (if (Variables|Default|GetSimulating)
    ;[0.15 0.15 0.15 0.5] Simulation Step
    (Development|PrintString "Step")
    (Class|SimulationLibrary|LBMHOMEStreamingCollision3D (Variables|Default|GetDisplaySlice))
    (Class|SimulationLibrary|GetDebugTextureValue3D (Variables|Default|GetOutDebugTex2D))))

(event Input|KeyboardEvents|DebugKey1
  (params (Key :type Key%20Structure :default "None") (ActionValue :type Input%20Action%20Value%20Structure))
  (:Pressed
    (Development|PrintString "Start Sim")
    (Variables|Default|SetSimulating true)))

(event Input|KeyboardEvents|DebugKey2
  (params (Key :type Key%20Structure :default "None") (ActionValue :type Input%20Action%20Value%20Structure))
  (:Pressed
    (Development|PrintString "Pause Sim")
    (Variables|Default|SetSimulating false)))

(event Input|KeyboardEvents|DebugKey3
  (params (Key :type Key%20Structure :default "None") (ActionValue :type Input%20Action%20Value%20Structure))
  (:Pressed
    ;[0.15 0.15 0.15 0.5] Simulation Step
    (Development|PrintString "Step")
    (Class|SimulationLibrary|LBMHOMEStreamingCollision3D (Variables|Default|GetDisplaySlice))
    (Class|SimulationLibrary|GetDebugTextureValue3D (Variables|Default|GetOutDebugTex2D))))

(event Input|KeyboardEvents|DebugKey0
  (params (Key :type Key%20Structure :default "None") (ActionValue :type Input%20Action%20Value%20Structure))
  (:Pressed
    (Class|SimulationLibrary|LBMMRInitialState3D (Variables|Default|GetDisplaySlice))
    ;[0.15 0.15 0.15 0.5] Reset Simulation Data
    (Class|SimulationLibrary|GetDebugTextureValue3D (Variables|Default|GetOutDebugTex2D))))

(fn ConstructionScript)